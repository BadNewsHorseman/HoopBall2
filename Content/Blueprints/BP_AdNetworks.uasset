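; BP_AdNetworks drives banner, interstitial and rewarded video ads through the UniversalMobileAds component.
; Each custom event walks its ad unit ID array in repeated passes, and the matching loaded callback breaks the loop.
; Interstitial and rewarded ads show as soon as they load, while banners are requested at the bottom of the screen.
; RewardClaimable is set when a video completes and cleared on close, with no reward granted here.
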(event BannerLoaded(UniversalMobileAds)
  (params (MediationResult :type Mediation%20Result%20Structure))
  (bind _banneradids (Variables|Default|GetBannerAdIDs))
  (Utilities|FlowControl|ForLoopwithBreak 0 2) ; enters at Break
)

(event InterstitialLoaded(UniversalMobileAds)
  (params (MediationResult :type Mediation%20Result%20Structure))
  (bind _interstitialadids (Variables|Default|GetInterstitialAdIDs))
  (Class|UniversalMobileAdsBlueprintLibrary|ShowInterstitial)
  (Utilities|FlowControl|ForLoopwithBreak 0 2) ; enters at Break
)

(event RewardedVideoLoadSuccess(UniversalMobileAds)
  (params (MediationResult :type Mediation%20Result%20Structure))
  (bind _rewardedadids (Variables|Default|GetRewardedAdIDs))
  (Class|UniversalMobileAdsBlueprintLibrary|ShowRewardedVideo)
  (Utilities|FlowControl|ForLoopwithBreak 0 2) ; enters at Break
)

(event RewardedVideoPlayingCompleted(UniversalMobileAds)
  (params (MediationResult :type Mediation%20Result%20Structure))
  (Variables|Default|SetRewardClaimable? true))

(event RewardedVideoClosed(UniversalMobileAds)
  (params (MediationResult :type Mediation%20Result%20Structure))
  (if (Variables|Default|GetRewardClaimable?)
    (Variables|Default|SetRewardClaimable? false)))

(event Custom|Banner
  (bind _banneradids (Variables|Default|GetBannerAdIDs))
  (Utilities|FlowControl|ForLoopwithBreak 0 2
    (:LoopBody
      (bind _index (Utilities|FlowControl|ForLoopwithBreak 0 (- (Utilities|Array|Length _banneradids) 1))
        (:LoopBody
          (Class|UniversalMobileAdsBlueprintLibrary|ShowBanner (Utilities|Array|Get(acopy) _banneradids _index) false))))))

(event Custom|Interstitial
  (bind _interstitialadids (Variables|Default|GetInterstitialAdIDs))
  (Utilities|FlowControl|ForLoopwithBreak 0 2
    (:LoopBody
      (bind _index (Utilities|FlowControl|ForLoopwithBreak 0 (- (Utilities|Array|Length _interstitialadids) 1))
        (:LoopBody
          (Class|UniversalMobileAdsBlueprintLibrary|LoadInterstitial (Utilities|Array|Get(acopy) _interstitialadids _index)))))))

(event Custom|Rewarded
  (bind _rewardedadids (Variables|Default|GetRewardedAdIDs))
  (Utilities|FlowControl|ForLoopwithBreak 0 2
    (:LoopBody
      (bind _index (Utilities|FlowControl|ForLoopwithBreak 0 (- (Utilities|Array|Length _rewardedadids) 1))
        (:LoopBody
          (Class|UniversalMobileAdsBlueprintLibrary|LoadRewardedVideo (Utilities|Array|Get(acopy) _rewardedadids _index)))))))

(event EventBeginPlay)

(fn ConstructionScript)