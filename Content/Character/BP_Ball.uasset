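; Player ball character that waits through a five-tick audio countdown at BeginPlay, then plays a GO sound and applies its gravity scale.
; D/A keys and MoveRight/MoveLeft events play or reverse a timeline that sets X position, each gated by a 0.1-second cooldown.
; A Move axis event adds movement input along world X.
; Touch-drag movement with position clamping and a fire-trail emitter are left disconnected and never run.
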(event Custom|TouchDrag)

(event Custom|Move
  (params (AxisValue :type Float%20%28single-precision%29))
  (Pawn|Input|AddMovementInput "1.000000, 0, 0" AxisValue false))

(event Custom|MouseOver)

(event Custom|MoveRight
  (bind _returnvalue (Transformation|GetActorLocation))
  (bind (_x _y _z) (Math|Vector|BreakVector _returnvalue))
  (if (Variables|Default|GetMovingR)
    (Utilities|FlowControl|Sequence
      (:then_0
        (Variables|Default|SetMovingR false)
        (bind _xlocation (Timeline|MoveRightLeft Play)
          (:Update
            (Transformation|SetActorLocation (Math|Vector|MakeVector _xlocation _y _z) false false))))
      (:then_1
        (Utilities|FlowControl|Delay 0.1)
        (Variables|Default|SetMovingR true)))))

(event Custom|MoveLeft
  (bind _returnvalue (Transformation|GetActorLocation))
  (bind (_x _y _z) (Math|Vector|BreakVector _returnvalue))
  (if (Variables|Default|GetMovingL)
    (Utilities|FlowControl|Sequence
      (:then_0
        (Variables|Default|SetMovingL false)
        (bind _xlocation (Timeline|MoveRightLeft Reverse)
          (:Update
            (Transformation|SetActorLocation (Math|Vector|MakeVector _xlocation _y _z) false false))))
      (:then_1
        (Utilities|FlowControl|Delay 0.1)
        (Variables|Default|SetMovingL true)))))

(event EventBeginPlay
  (Variables|/Script/Engine.PlayerController|SetbShowMouseCursor (Game|GetPlayerController 0) true)
  (Transformation|SetActorLocation "-72.500000, 0,250.000000" false false)
  (Utilities|FlowControl|Delay 1.0)
  (Audio|PlaySound2D "/Game/Interface_and_Item_SFX_10/MISC/wav/Countdown__5__Tick.Countdown__5__Tick" 1.0 1.0 0.0 0 0)
  (Math|Integer|DecrementInt (Variables|Default|Getcountdowntimeleft)
    (:%20%20
      (Utilities|FlowControl|Delay 1.0)
      (Audio|PlaySound2D "/Game/Interface_and_Item_SFX_10/MISC/wav/Countdown__5__Tick.Countdown__5__Tick" 1.0 1.0 0.0 0 0)
      (Math|Integer|DecrementInt (Variables|Default|Getcountdowntimeleft)
        (:%20%20
          (Utilities|FlowControl|Delay 1.0)
          (Audio|PlaySound2D "/Game/Interface_and_Item_SFX_10/MISC/wav/Countdown__5__Tick.Countdown__5__Tick" 1.0 1.0 0.0 0 0)
          (Math|Integer|DecrementInt (Variables|Default|Getcountdowntimeleft)
            (:%20%20
              (Utilities|FlowControl|Delay 1.0)
              (Audio|PlaySound2D "/Game/Interface_and_Item_SFX_10/MISC/wav/Countdown__5__Tick.Countdown__5__Tick" 1.0 1.0 0.0 0 0)
              (Math|Integer|DecrementInt (Variables|Default|Getcountdowntimeleft)
                (:%20%20
                  (Utilities|FlowControl|Delay 1.0)
                  (Audio|PlaySound2D "/Game/Interface_and_Item_SFX_10/MISC/wav/Countdown__5__Tick.Countdown__5__Tick" 1.0 1.0 0.0 0 0)
                  (Math|Integer|DecrementInt (Variables|Default|Getcountdowntimeleft)
                    (:%20%20
                      (Audio|PlaySound2D "/Game/Interface_and_Item_SFX_10/MISC/wav/Countdown_GO__2_.Countdown_GO__2_" 1.0 1.0 0.0 0 0)
                      (Variables|/Script/Engine.CharacterMovementComponent|SetGravityScale (Variables|Character|GetCharacterMovement) (Variables|Default|GetGravityScale)))))))))))))

(event Input|AxisEvents|InputAxisMoveRight
  (params (AxisValue :type Float%20%28single-precision%29)))

(event Input|KeyboardEvents|D
  (params (Key :type Key%20Structure))
  (bind _returnvalue (Transformation|GetActorLocation))
  (bind (_x _y _z) (Math|Vector|BreakVector _returnvalue))
  (:Pressed
    (if (Variables|Default|GetMovingR)
      (Utilities|FlowControl|Sequence
        (:then_0
          (Variables|Default|SetMovingR false)
          (bind _xlocation (Timeline|MoveRightLeft Play)
            (:Update
              (Transformation|SetActorLocation (Math|Vector|MakeVector _xlocation _y _z) false false))))
        (:then_1
          (Utilities|FlowControl|Delay 0.1)
          (Variables|Default|SetMovingR true))))))

(event Input|KeyboardEvents|A
  (params (Key :type Key%20Structure))
  (bind _returnvalue (Transformation|GetActorLocation))
  (bind (_x _y _z) (Math|Vector|BreakVector _returnvalue))
  (:Pressed
    (if (Variables|Default|GetMovingL)
      (Utilities|FlowControl|Sequence
        (:then_0
          (Variables|Default|SetMovingL false)
          (bind _xlocation (Timeline|MoveRightLeft Reverse)
            (:Update
              (Transformation|SetActorLocation (Math|Vector|MakeVector _xlocation _y _z) false false))))
        (:then_1
          (Utilities|FlowControl|Delay 0.1)
          (Variables|Default|SetMovingL true))))))

(event Input|TouchEvents|InputTouch
  (params (Location :type Vector) (FingerIndex :type ETouchIndex%20Enum)))

(fn ConstructionScript)