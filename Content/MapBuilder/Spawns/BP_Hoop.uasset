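; BP_Hoop is a scoring hoop that grants a random point value to a BP_Ball passing through it.
; On BeginPlay it picks the value from PointsToGrant and shows it on its TextRender.
; Any Box overlap plays a random sound and lightning effect; only a ball then gains the points and destroys the hoop.
; The sound index range includes the array length, so it can land out of bounds.
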(event OnComponentBeginOverlap(Box)
  (params (OverlappedComponent :type Primitive%20Component%20Object%20Reference) (OtherActor :type Actor%20Object%20Reference) (OtherComp :type Primitive%20Component%20Object%20Reference) (OtherBodyIndex :type Integer) (bFromSweep :type Boolean) (SweepResult :type Hit%20Result%20Structure%20%28by%20ref%29))
  (bind _sound_toplay (Variables|Default|Getsound%20toplay))
  (Audio|PlaySound2D (Utilities|Array|Get(acopy) _sound_toplay (Math|Random|RandomIntegerinRange 0 (Utilities|Array|Length _sound_toplay))) 1.0 1.0 0.0 0 0)
  (Effects|SpawnEmitteratLocation "/Game/Cartoony_Impact_-_Stylized_Particle_Simulation_1/Particles/PS_Lightning2.PS_Lightning2" (Transformation|GetWorldLocation (Variables|Default|GetBox)))
  (bind _asbp_ball (Utilities|Casting|CastToBP_Ball OtherActor))
  (Variables|/Game/Character/BP_Ball.BP_Ball_C|SetScore _asbp_ball (+ (Variables|/Game/Character/BP_Ball.BP_Ball_C|GetScore _asbp_ball) (Variables|Default|GetPoints)))
  (Actor|DestroyActor))

(event EventBeginPlay
  (bind _pointstogrant (Variables|Default|GetPointsToGrant))
  (bind _output_get (Variables|Default|SetPoints (Utilities|Array|Get(acopy) _pointstogrant (Math|Random|RandomIntegerinRange 0 (- (Utilities|Array|Length _pointstogrant) 1)))))
  (Rendering|Components|TextRender|SetText (Variables|Default|GetTextRender) (Utilities|Text|ToText(String) (Utilities|String|Append (Utilities|String|ToString(Integer) _output_get) " Points"))))

(event Collision|EventActorBeginOverlap
  (params (OtherActor :type Actor%20Object%20Reference)))

(event EventTick
  (params (DeltaSeconds :type Float%20%28single-precision%29)))

(fn ConstructionScript)